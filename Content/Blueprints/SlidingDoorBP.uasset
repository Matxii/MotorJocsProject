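; Key-locked sliding door with a console that displays how many keys it requires.
; When the first-person character enters the door collider, it asks the game instance to consume the keys and, on success, plays a timeline that offsets the mesh vertically from its initial position.
; Leaving reverses the timeline, and each re-entry attempts to consume keys again.
; Overlapping the console collider shows the key count as two-digit text, hidden otherwise.
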(event `self.ReceiveBeginPlay`
  (set `self.DoorRelativePosInit` (`SceneComponent.RelativeLocation` (`self.DoorSM`)))
  (`SceneComponent.SetVisibility` (`self.TextRender`) false false))

(event `self.DoorCollider.OnComponentBeginOverlap`
  (params (OverlappedComponent :type "PrimitiveComponent Object Reference") (OtherActor :type "Actor Object Reference") (OtherComp :type "PrimitiveComponent Object Reference") (OtherBodyIndex :type Integer) (bFromSweep :type Boolean) (SweepResult :type "HitResult Structure (by ref)"))
  (cast `/Game/FirstPersonBP/Blueprints/FirstPersonCharacter` OtherActor)
  (bind _success (`/Game/Blueprints/Game/MyGameInstanceBP.ConsumeKeys` (cast `/Game/Blueprints/Game/MyGameInstanceBP` (`GameplayStatics.GetGameInstance`) :!pure true) (`self.NumKeys`)))
  (if _success
    (bind (_direction _zoffset) (`Timeline|SlidingDoorTL` :!label _label)
      (:`Update`
        (`SceneComponent.K2_SetRelativeLocation` (`self.DoorSM`) (+ (`KismetMathLibrary.MakeVector` 0.0 0.0 _zoffset) (`self.DoorRelativePosInit`)) false false)))))

(event `self.DoorCollider.OnComponentEndOverlap`
  (params (OverlappedComponent :type "PrimitiveComponent Object Reference") (OtherActor :type "Actor Object Reference") (OtherComp :type "PrimitiveComponent Object Reference") (OtherBodyIndex :type Integer))
  (cast `/Game/FirstPersonBP/Blueprints/FirstPersonCharacter` OtherActor)
  (goto _label :!via `Reverse`))

(event `self.ConsoleCollider.OnComponentBeginOverlap`
  (params (OverlappedComponent :type "PrimitiveComponent Object Reference") (OtherActor :type "Actor Object Reference") (OtherComp :type "PrimitiveComponent Object Reference") (OtherBodyIndex :type Integer) (bFromSweep :type Boolean) (SweepResult :type "HitResult Structure (by ref)"))
  (cast `/Game/FirstPersonBP/Blueprints/FirstPersonCharacter` OtherActor)
  (`TextRenderComponent.K2_SetText` (`self.TextRender`) (`KismetTextLibrary.Conv_IntToText` (`self.NumKeys`) true 2 2))
  (`SceneComponent.SetVisibility` (`self.TextRender`) true false))

(event `self.ConsoleCollider.OnComponentEndOverlap`
  (params (OverlappedComponent :type "PrimitiveComponent Object Reference") (OtherActor :type "Actor Object Reference") (OtherComp :type "PrimitiveComponent Object Reference") (OtherBodyIndex :type Integer))
  (cast `/Game/FirstPersonBP/Blueprints/FirstPersonCharacter` OtherActor)
  (`SceneComponent.SetVisibility` (`self.TextRender`) false false))

(fn `UserConstructionScript`)