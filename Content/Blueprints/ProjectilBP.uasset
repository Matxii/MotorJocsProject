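; Projectile Blueprint that launches itself on spawn and explodes when it hits an actor of a particular type.
; On BeginPlay it adds a velocity-change impulse to its physics-driven static mesh, built from its Direction and Impulse variables.
; A component hit that passes the cast check spawns an explosion emitter at the impact point, plays a lower-pitched explosion sound and destroys the projectile.
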(event `self.ReceiveBeginPlay`
  (`PrimitiveComponent.AddImpulse` (`self.StaticMesh`) (* (`self.Direction`) (`self.Impulse`)) "None" true))

(event `self.StaticMesh.OnComponentHit`
  (params (HitComponent :type "PrimitiveComponent Object Reference") (OtherActor :type "Actor Object Reference") (OtherComp :type "PrimitiveComponent Object Reference") (NormalImpulse :type "Vector Structure") (Hit :type "HitResult Structure (by ref)"))
  (cast `` OtherActor)
  (`GameplayStatics.SpawnEmitterAtLocation` "/Game/StarterContent/Particles/P_Explosion.P_Explosion" (`.Location` (`GameplayStatics.BreakHitResult` Hit)))
  (`GameplayStatics.SpawnSoundAtLocation` "/Game/StarterContent/Audio/Explosion01.Explosion01" (0.0 0.0 0.0) (struct) 1.0 0.5)
  (`self.K2_DestroyActor`))

(fn `UserConstructionScript`)