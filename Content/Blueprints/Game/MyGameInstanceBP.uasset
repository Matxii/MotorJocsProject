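; MyGameInstanceBP is a Game Instance Blueprint that tracks the key count in an Inventory struct.
; AddKeys increases NumKeys by the given amount.
; ConsumeKeys subtracts the requested amount and returns true only when enough keys are held, otherwise returning false with the count unchanged.
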(fn `AddKeys`
  (params (NumKeys :type Integer))
  (setmembers `/Game/Blueprints/Game/SInventory` :`StructRef` (`self.Inventory`) :`NumKeys` (+ NumKeys (`.NumKeys_2_363995344A89B99F24BFD99BBF8E8A0C` (break `/Game/Blueprints/Game/SInventory` (`self.Inventory`)))))
  (return))

(fn `ConsumeKeys`
  (params (NumKeys :type Integer))
  (returns (Success :type Boolean))
  (if (<= NumKeys (`.NumKeys_2_363995344A89B99F24BFD99BBF8E8A0C` (break `/Game/Blueprints/Game/SInventory` (`self.Inventory`))))
    (setmembers `/Game/Blueprints/Game/SInventory` :`StructRef` (`self.Inventory`) :`NumKeys` (- (`.NumKeys_2_363995344A89B99F24BFD99BBF8E8A0C` (break `/Game/Blueprints/Game/SInventory` (`self.Inventory`))) NumKeys))
    (return true)
    (else
      (return false))))