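; Game mode that switches the game between main menu, in-play and pause states, starting at the main menu on BeginPlay.
; A ChangeGameModeEtv event calls a function for each requested state and records it, ignoring pause requests while already paused.
; Each function adds or removes the menu widgets and sets cursor and input mode, with pause and resume also toggling game pause.
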(event `self.ReceiveBeginPlay`
  (`self.ChangeGameModeEtv` "NewEnumerator0"))

(event `ChangeGameModeEtv`
  (params (`New Mode` :type "/Game/Blueprints/Game/EGameModes_MJ Enum" :default "NewEnumerator0"))
  (switch `/Game/Blueprints/Game/EGameModes_MJ` `New Mode`
    (:`NewEnumerator0`
      (`self.MainMenu`)
      (set `self.GameMode` `New Mode` :!label _label))
    (:`NewEnumerator1`
      (`self.InPlay`)
      (goto _label))
    (:`NewEnumerator2`
      (if (not (`GameplayStatics.IsGamePaused`))
        (`self.PauseMenu`)
        (goto _label)))))

(fn `InPlay`
  (bind _returnvalue (`GameplayStatics.GetPlayerController` 0))
  (if (`GameplayStatics.IsGamePaused`)
    (`GameplayStatics.SetGamePaused` false))
  (`|ExecutionSequence`
    (:`then_0`
      (if (!= (`self.MyMainMenuWB`) null)
        (`Widget.RemoveFromParent` (`self.MyMainMenuWB`)))
      (set `PlayerController.bShowMouseCursor` false _returnvalue)
      (`WidgetBlueprintLibrary.SetInputMode_GameOnly` _returnvalue))
    (:`then_1`
      (if (!= (`self.MyPauseMenuWB`) null)
        (`Widget.RemoveFromParent` (`self.MyPauseMenuWB`))))))

(fn `MainMenu`
  (bind _returnvalue (`GameplayStatics.GetPlayerController` 0))
  (if (!= (`self.MyPauseMenuWB`) null)
    (`Widget.RemoveFromParent` (`self.MyPauseMenuWB`)))
  (bind _returnvalue_2 (`|CreateWidget` "/Game/Blueprints/Game/UMG/MainMenu_MJ.MainMenu_MJ_C" _returnvalue))
  (bind _output_get (set `self.MyMainMenuWB` _returnvalue_2))
  (`UserWidget.AddToViewport` _output_get 0)
  (`WidgetBlueprintLibrary.SetInputMode_UIOnlyEx` _returnvalue)
  (set `PlayerController.bShowMouseCursor` true _returnvalue))

(fn `PauseMenu`
  (bind _returnvalue (`GameplayStatics.GetPlayerController` 0))
  (bind _returnvalue_2 (`|CreateWidget` "/Game/Blueprints/Game/UMG/PauseMenu_MJ.PauseMenu_MJ_C" _returnvalue))
  (bind _output_get (set `self.MyPauseMenuWB` _returnvalue_2))
  (`UserWidget.AddToViewport` _output_get 0)
  (`GameplayStatics.SetGamePaused` true)
  (set `PlayerController.bShowMouseCursor` true _returnvalue)
  (`WidgetBlueprintLibrary.SetInputMode_UIOnlyEx` _returnvalue))

(fn `UserConstructionScript`)