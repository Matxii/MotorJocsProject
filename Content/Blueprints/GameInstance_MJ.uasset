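; GameInstance_MJ is a game instance Blueprint that holds the player's star count inside an InventoryMJ struct for the whole session.
; AddStar increases the stored star total by a given amount.
; ConsumeStar deducts stars only when the inventory holds enough and returns whether the spend succeeded.
; Both functions write back through a set-members operation on the struct; no saving is shown here.
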(fn `AddStar`
  (params (Stars :type Integer :default 5))
  (setmembers `/Game/Blueprints/PInventory` :`StructRef` (`self.Inventory_MJ`) :`Stars` (+ Stars (`.Stars_4_091477E54FCD9064D7484994C4C1674B` (break `/Game/Blueprints/PInventory` (`self.Inventory_MJ`)))))
  (return))

(fn `ConsumeStar`
  (params (Stars :type Integer))
  (returns (Success :type Boolean))
  (if (<= Stars (`.Stars_4_091477E54FCD9064D7484994C4C1674B` (break `/Game/Blueprints/PInventory` (`self.Inventory_MJ`))))
    (setmembers `/Game/Blueprints/PInventory` :`StructRef` (`self.Inventory_MJ`) :`Stars` (- (`.Stars_4_091477E54FCD9064D7484994C4C1674B` (break `/Game/Blueprints/PInventory` (`self.Inventory_MJ`))) Stars))
    (return true)
    (else
      (return false))))