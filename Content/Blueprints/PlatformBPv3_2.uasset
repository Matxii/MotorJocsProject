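; Moving platform actor that slides its static mesh along the actor's forward vector.
; On BeginPlay it stores the starting location and calls a custom movement event that plays a timeline from the start.
; Each timeline update multiplies the curve value by an Offset variable and sets the mesh's world location relative to the start, without sweep.
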(event `MovementEvt`
  (bind (_direction _offset) (`Timeline|MovementTL` :!via `PlayFromStart`)
    (:`Update`
      (`SceneComponent.K2_SetWorldLocation` (`self.PlatformSM`) (+ (* (`self.GetActorForwardVector`) (* _offset (`self.Offset`))) (`self.InitPos`)) false false))))

(event `self.ReceiveBeginPlay`
  (set `self.InitPos` (`self.K2_GetActorLocation`))
  (`self.MovementEvt`))

(fn `UserConstructionScript`)