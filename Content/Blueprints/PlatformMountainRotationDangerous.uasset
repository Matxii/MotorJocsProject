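; A dangerous platform that fades away and destroys itself if the player character stays on it too long.
; The construction script gives the platform mesh a dynamic material instance for controlling opacity.
; When the character enters the box, a timeline plays in reverse from its end, driving opacity and a visible countdown text, then destroys the actor.
; Leaving early stops the timeline, restores full opacity and hides the text.
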(event `self.Box.OnComponentBeginOverlap`
  (params (OverlappedComponent :type "PrimitiveComponent Object Reference") (OtherActor :type "Actor Object Reference") (OtherComp :type "PrimitiveComponent Object Reference") (OtherBodyIndex :type Integer) (bFromSweep :type Boolean) (SweepResult :type "HitResult Structure (by ref)"))
  (cast `/Game/Mannequin/Character_Blueprint_MJ` OtherActor)
  (bind (_direction _opacity) (`Timeline|OpacityTL` :!via `ReverseFromEnd`)
    (:`Update`
      (`MaterialInstanceDynamic.SetScalarParameterValue` (`self.Material`) "Opacity" _opacity)
      (`TextRenderComponent.K2_SetText` (`self.Text`) (`KismetTextLibrary.Conv_DoubleToText` (`TimelineComponent.GetPlaybackPosition` (`self.OpacityTL`)) "HalfToEven"))
      (`SceneComponent.SetVisibility` (`self.Text`) true false))
    (:`Finished`
      (`self.K2_DestroyActor`))))

(event `self.Box.OnComponentEndOverlap`
  (params (OverlappedComponent :type "PrimitiveComponent Object Reference") (OtherActor :type "Actor Object Reference") (OtherComp :type "PrimitiveComponent Object Reference") (OtherBodyIndex :type Integer))
  (cast `/Game/Mannequin/Character_Blueprint_MJ` OtherActor)
  (`TimelineComponent.Stop` (`self.OpacityTL`))
  (`MaterialInstanceDynamic.SetScalarParameterValue` (`self.Material`) "Opacity" 1.0)
  (`SceneComponent.SetVisibility` (`self.Text`) false false))

(fn `UserConstructionScript`
  (bind _returnvalue (`KismetMaterialLibrary.CreateDynamicMaterialInstance` "/Game/Blueprints/Materials/PlatformOpacityMAT_Inst.PlatformOpacityMAT_Inst"))
  (bind _output_get (set `self.Material` _returnvalue))
  (`PrimitiveComponent.SetMaterial` (`self.Platform SM`) 0 _output_get))