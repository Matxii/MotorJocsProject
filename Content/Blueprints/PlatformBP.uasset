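; A moving platform Blueprint whose static mesh oscillates back and forth around the world location it had at BeginPlay.
; Each Tick offsets that start point by a game-time sine wave, using Periodo as the period and Recorrido as the amplitude.
; SentidoMovimiento selects world X or Y as the axis, and the mesh moves without sweep.
; Component hits on the mesh only print the hit distance.
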(event `self.ReceiveBeginPlay`
  (set `self.PosicionInicial` (`SceneComponent.K2_GetComponentLocation` (`self.StaticMesh`))))

(event `self.ReceiveTick`
  (params (DeltaSeconds :type "Float (single-precision)"))
  (bind _posicioninicial (`self.PosicionInicial`))
  (bind _staticmesh (`self.StaticMesh`))
  (bind _returnvalue (* (`KismetMathLibrary.Sin` (/ (* (`KismetSystemLibrary.GetGameTimeInSeconds`) 6.3) (`self.Periodo`))) (`self.Recorrido`)))
  (switch `/Game/Blueprints/ESentidoPlataforma` (`self.SentidoMovimiento`)
    (:`NewEnumerator0`
      (`SceneComponent.K2_SetWorldLocation` _staticmesh (+ _posicioninicial (`KismetMathLibrary.MakeVector` _returnvalue)) false false))
    (:`NewEnumerator1`
      (`SceneComponent.K2_SetWorldLocation` _staticmesh (+ _posicioninicial (`KismetMathLibrary.MakeVector` 0.0 _returnvalue)) false false))))

(event `self.StaticMesh.OnComponentHit`
  (params (HitComponent :type "PrimitiveComponent Object Reference") (OtherActor :type "Actor Object Reference") (OtherComp :type "PrimitiveComponent Object Reference") (NormalImpulse :type "Vector Structure") (Hit :type "HitResult Structure (by ref)"))
  (`KismetSystemLibrary.PrintString` (`KismetStringLibrary.Conv_DoubleToString` (`.Distance` (`GameplayStatics.BreakHitResult` Hit))) true false))

(fn `UserConstructionScript`)